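; BP_TestGrid is a test actor in the AI folder that visualizes a tiled ground grid with debug drawing.
; Its construction script flushes old debug lines, then draws the grid bounds, a bottom-left corner marker and the tiles.
; DrawTile derives tile counts from GridSizeWorld and TileSize, both treated as half-extents, and lays planes along the actor's right and forward vectors.
; The bounds box stays world-axis aligned, and gameplay events are empty.
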(event EventBeginPlay)

(event Collision|EventActorBeginOverlap
  (params (OtherActor :type Actor%20Object%20Reference)))

(event EventTick
  (params (DeltaSeconds :type Float%20%28single-precision%29)))

(fn ConstructionScript
  (bind _gridsizeworld (Variables|Grid|GetGridSizeWorld))
  (Rendering|Debug|FlushPersistentDebugLines)
  (Variables|Grid|SetGridLocation (Transformation|GetWorldLocation (Variables|Default|GetScene)))
  (Rendering|Debug|DrawDebugBox (Variables|Grid|GetGridLocation) (Math|Vector|MakeVector (.y _gridsizeworld) (.x _gridsizeworld) 5.0) (Variables|Debug|GetGridBoxColor) "0, 0, 0" 1e+06 5.0)
  (Rendering|Debug|DrawDebugBox (CallFunction|GridBottomLeft) (Math|Vector|MakeVector 5.0 5.0 5.0) (Variables|Default|GetBottomLeftColor) "0, 0, 0" 1e+06 5.0)
  (CallFunction|DrawTile))

(fn GridBottomLeft
  (return (- (- (Variables|Grid|GetGridLocation) (* (Math|Vector|GetRightVector (Variables|Default|GetScene)) (.x (Variables|Grid|GetGridSizeWorld)))) (* (Math|Vector|GetForwardVector (Variables|Default|GetScene)) (.y (Variables|Grid|GetGridSizeWorld))))))

(fn GridTileNumber
  (bind _gridsizeworld (Variables|Grid|GetGridSizeWorld))
  (bind _tilesize (Variables|Grid|GetTileSize))
  (return (- (Math|Float|Round (/ (.x _gridsizeworld) _tilesize)) 1) (- (Math|Float|Round (/ (.y _gridsizeworld) _tilesize)) 1)))

(fn DrawTile
  (bind (_gridtilenumberx _gridtilenumbery) (CallFunction|GridTileNumber))
  (bind _tilesize (Variables|Grid|GetTileSize))
  (bind _tilesize_2 (Variables|Grid|GetTileSize))
  (for _index (range 0 _gridtilenumberx)
    (LocalVariables|SetX _index)
    (for _index_2 (range 0 _gridtilenumbery)
      (LocalVariables|SetY _index_2)
      (bind _output_get (LocalVariables|SetTilePosition (+ (CallFunction|GridBottomLeft) (* (Math|Vector|GetRightVector (Variables|Default|GetScene)) (+ (* (LocalVariables|GetX) (* _tilesize 2.0)) _tilesize)) (* (Math|Vector|GetForwardVector (Variables|Default|GetScene)) (+ (* (LocalVariables|GetY) (* _tilesize_2 2.0)) _tilesize_2)))))
      (Class|KismetSystemLibrary|DrawDebugPlane (Utilities|Struct|MakePlane (.Z (Math|Vector|BreakVector _output_get)) 0.0 0.0 1.0) _output_get (- (Variables|Grid|GetTileSize) 5.0) "(R=0.103126,G=0.765625,B=0.037601,A=1.000000)" 1e+05))))