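; Navigation grid actor for DinnerOrDiner AI that previews its layout through debug drawing.
; The construction script flushes persistent debug lines, then calls DrawShape and DrawTile, or destroys the actor if it is invalid.
; On BeginPlay it only prints the Scene component's world location and a GridLocation value to check placement.
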(event EventBeginPlay
  (Development|PrintString (Utilities|String|ToString(Vector) (Transformation|GetWorldLocation (Variables|Default|GetScene))))
  (Development|PrintString (Utilities|String|ToString(Vector) (Variables|/Script/DinnerOrDiner_UE.DinnerOrDiner_NavGrid|GetGridLocation (Variables|Default|GetGetter)))))

(event Collision|EventActorBeginOverlap
  (params (OtherActor :type Actor%20Object%20Reference)))

(event EventTick
  (params (DeltaSeconds :type Float%20%28single-precision%29)))

(fn ConstructionScript
  (Utilities|IsValid self
    (:Is%20Valid
      (Rendering|Debug|FlushPersistentDebugLines)
      (Class|DinnerorDinerNavGrid|DrawShape)
      (Class|DinnerorDinerNavGrid|DrawTile))
    (:Is%20Not%20Valid
      (Rendering|Debug|FlushPersistentDebugLines)
      (Actor|DestroyActor))))